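; Player controller for mouse-driven movement and attacks on BP_Character.
; Holding the right mouse button opens a Tick gate that continuously moves the pawn toward the hit location under the cursor.
; Without authority, it sends the goal through a server move event and also runs SimpleMoveToLocation locally.
; Left click casts player character 0 to BP_Character and calls AttackCombo.
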(event `Server_Move`
  (params (Controller :type "Controller Object Reference") (Goal :type "Vector Structure (by ref)"))
  (`AIBlueprintHelperLibrary.SimpleMoveToLocation` Controller Goal))

(event `self.ReceiveTick`
  (params (DeltaSeconds :type "Float (single-precision)"))
  (`/Engine/EditorBlueprintResources/StandardMacros.Gate` true :!label _label
    (:`Exit`
      (set `self.Location` (`.Location` (`GameplayStatics.BreakHitResult` (`self.GetHitResultUnderCursorByChannel` "TraceTypeQuery1"))))
      (`/Engine/EditorBlueprintResources/ActorMacros.Switch Has Authority`
        (:`Authority`
          (`AIBlueprintHelperLibrary.SimpleMoveToLocation` self (`self.Location`)))
        (:`Remote`
          (`self.Server_Move` self (`self.Location`))
          (`AIBlueprintHelperLibrary.SimpleMoveToLocation` self (`self.Location`)))))))

(event `Key|RightMouseButton`
  (params (Key :type "Key Structure"))
  (:`Pressed`
    (goto _label :!via `Open`))
  (:`Released`
    (goto _label :!via `Close`)))

(event `Key|LeftMouseButton`
  (params (Key :type "Key Structure"))
  (:`Pressed`
    (bind _asbp_character (cast `/Game/_Game/BP_Character` (`GameplayStatics.GetPlayerCharacter` 0)))
    (`/Game/_Game/BP_Character.AttackCombo` _asbp_character)))

(fn `UserConstructionScript`)